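; Portal gun manager that places linked blue (left) and yellow (right) portals where the player's camera aims, reacting to FirstPersonCharacter dispatchers.
; Each spawn line-traces to a surface, replaces that side's previous portal, links targets and plays a scale-opening timeline.
; InitializeSceneCapture shows the opposite portal's capture through a viewport-sized render target and dynamic material.
; UpdatePortal computes view-relative camera transforms and clip planes, but its calls are disconnected from Tick.
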(event `self.ReceiveBeginPlay`
  (add `/Game/Blueprints/FirstPersonCharacter.BluePortalDispatcher` (cast `/Game/Blueprints/FirstPersonCharacter` (`GameplayStatics.GetPlayerCharacter` 0) :!pure true) (delegate `BluePortalCustomEvent`))
  (add `/Game/Blueprints/FirstPersonCharacter.YellowPortalDispatcher` (cast `/Game/Blueprints/FirstPersonCharacter` (`GameplayStatics.GetPlayerCharacter` 0) :!pure true) (delegate `YellowPortalCustomEvent`)))

(event `BluePortalCustomEvent`
  (bind _right_ptl (`self.Right_PTL`))
  (bind _leftportal (`self.Spawn Portal 1`))
  (`self.InitializeSceneCapture` _leftportal (`self.Right_PTL`))
  (`/Engine/EditorBlueprintResources/StandardMacros.IsValid` _right_ptl
    (:`Is Valid`
      (`self.InitializeSceneCapture` _right_ptl (`self.Left_PTL`))
      (bind (_direction _portal_opening) (`Timeline|OpenPortal 1` :!via `PlayFromStart` :!label _label)
        (:`Update`
          (bind _returnvalue_x (`KismetMathLibrary.BreakVector` (`self.GetActorScale3D` _leftportal)))
          (`self.SetActorScale3D` _leftportal (`KismetMathLibrary.MakeVector` _returnvalue_x _portal_opening _portal_opening)))))
    (:`Is Not Valid`
      (goto _label :!via `PlayFromStart`))))

(event `YellowPortalCustomEvent`
  (bind _left_ptl (`self.Left_PTL`))
  (bind _rightportal (`self.Spawn Portal 2`))
  (`self.InitializeSceneCapture` _rightportal _left_ptl)
  (`/Engine/EditorBlueprintResources/StandardMacros.IsValid` _left_ptl
    (:`Is Valid`
      (`self.InitializeSceneCapture` _left_ptl (`self.Right_PTL`))
      (bind (_direction _portal_opening) (`Timeline|OpenPortal` :!via `PlayFromStart` :!label _label_2)
        (:`Update`
          (bind _returnvalue_x (`KismetMathLibrary.BreakVector` (`self.GetActorScale3D` _rightportal)))
          (`self.SetActorScale3D` _rightportal (`KismetMathLibrary.MakeVector` _returnvalue_x _portal_opening _portal_opening)))))
    (:`Is Not Valid`
      (goto _label_2 :!via `PlayFromStart`))))

(event `self.ReceiveTick`
  (params (DeltaSeconds :type "Float (single-precision)")))

(fn `InitializeSceneCapture`
  (params (ThisPortal :type "/Game/Blueprints/BP_Portal Object Reference") (OtherPortal :type "/Game/Blueprints/BP_Portal Object Reference"))
  (bind (_returnvalue_x _returnvalue_y) (`KismetMathLibrary.BreakVector2D` (`WidgetLayoutLibrary.GetViewportSize`)))
  (bind _returnvalue (`KismetRenderingLibrary.CreateRenderTarget2D` (`KismetMathLibrary.FTrunc` _returnvalue_x) (`KismetMathLibrary.FTrunc` _returnvalue_y)))
  (bind _output_get (set `self.RenderTarget` _returnvalue))
  (`/Engine/EditorBlueprintResources/StandardMacros.IsValid` OtherPortal
    (:`Is Valid`
      (set `SceneCaptureComponent2D.TextureTarget` _output_get (`/Game/Blueprints/BP_Portal.PortalCam` OtherPortal)))
    (:`Is Not Valid`
      (set `SceneCaptureComponent2D.TextureTarget` _output_get (`/Game/Blueprints/BP_Portal.PortalCam` ThisPortal))))
  (bind _returnvalue_2 (`PrimitiveComponent.CreateDynamicMaterialInstance` (`/Game/Blueprints/BP_Portal.MeshP` ThisPortal) 0 "/Game/Materials/Portal_Mat.Portal_Mat" "None"))
  (`MaterialInstanceDynamic.SetTextureParameterValue` _returnvalue_2 "TextureRT" (`self.RenderTarget`)))

(fn `Spawn Portal 1`
  (returns (LeftPortal :type "/Game/Blueprints/BP_LeftPortal Object Reference"))
  (bind _right_ptl (`self.Right_PTL`))
  (bind _playercameramanager (`PlayerController.PlayerCameraManager` (`GameplayStatics.GetPlayerController` 0)))
  (bind _returnvalue (`PlayerCameraManager.GetCameraLocation` _playercameramanager))
  (bind _outhit (`KismetSystemLibrary.LineTraceSingle` _returnvalue (+ (* (`KismetMathLibrary.GetForwardVector` (`PlayerCameraManager.GetCameraRotation` _playercameramanager)) 10000.0) _returnvalue) "TraceTypeQuery1"))
  (`KismetSystemLibrary.PrintString` (`KismetStringLibrary.Conv_VectorToString` (`.ImpactNormal` (`GameplayStatics.BreakHitResult` _outhit))) true true (struct :`G` 0.66 :`B` 1.0 :`A` 1.0) 10.0)
  (`/Engine/EditorBlueprintResources/StandardMacros.IsValid` (`self.Left_PTL`)
    (:`Is Valid`
      (`self.K2_DestroyActor` (`self.Left_PTL`))
      (`KismetSystemLibrary.PrintString` "Destroy!"))
    (:`Is Not Valid`
      _))
  (bind _returnvalue_2 (`|SpawnActorFromClass` "/Game/Blueprints/BP_LeftPortal.BP_LeftPortal_C" (`KismetMathLibrary.MakeTransform` (+ (`.ImpactPoint` (`GameplayStatics.BreakHitResult` _outhit)) (* (`.ImpactNormal` (`GameplayStatics.BreakHitResult` _outhit)) 0.01)) (`KismetMathLibrary.Conv_VectorToRotator` (`.ImpactNormal` (`GameplayStatics.BreakHitResult` _outhit))) (1.0 0.2 0.2)) "Undefined" "OverrideRootScale" null null null))
  (bind _output_get (set `self.Left_PTL` _returnvalue_2))
  (set `self.Portal_1` _output_get)
  (`/Engine/EditorBlueprintResources/StandardMacros.IsValid` _right_ptl
    (:`Is Valid`
      (set `/Game/Blueprints/BP_Portal.TargetPortal` _right_ptl _output_get)
      (set `/Game/Blueprints/BP_Portal.TargetPortal` _output_get (`self.Right_PTL`)))
    (:`Is Not Valid`
      _))
  (return _output_get))

(fn `Spawn Portal 2`
  (returns (RightPortal :type "/Game/Blueprints/BP_RightPortal Object Reference"))
  (bind _left_ptl (`self.Left_PTL`))
  (bind _playercameramanager (`PlayerController.PlayerCameraManager` (`GameplayStatics.GetPlayerController` 0)))
  (bind _returnvalue (`PlayerCameraManager.GetCameraLocation` _playercameramanager))
  (bind _outhit (`KismetSystemLibrary.LineTraceSingle` _returnvalue (+ (* (`KismetMathLibrary.GetForwardVector` (`PlayerCameraManager.GetCameraRotation` _playercameramanager)) 10000.0) _returnvalue) "TraceTypeQuery1"))
  (`/Engine/EditorBlueprintResources/StandardMacros.IsValid` (`self.Right_PTL`)
    (:`Is Valid`
      (`self.K2_DestroyActor` (`self.Right_PTL`))
      (`KismetSystemLibrary.PrintString` "Destroy!"))
    (:`Is Not Valid`
      _))
  (bind _returnvalue_2 (`|SpawnActorFromClass` "/Game/Blueprints/BP_RightPortal.BP_RightPortal_C" (`KismetMathLibrary.MakeTransform` (+ (`.ImpactPoint` (`GameplayStatics.BreakHitResult` _outhit)) (* (`.ImpactNormal` (`GameplayStatics.BreakHitResult` _outhit)) 0.01)) (`KismetMathLibrary.Conv_VectorToRotator` (`.ImpactNormal` (`GameplayStatics.BreakHitResult` _outhit))) (1.0 0.2 0.2)) "Undefined" "OverrideRootScale" null null null))
  (bind _output_get (set `self.Right_PTL` _returnvalue_2))
  (set `self.Portal_2` _output_get)
  (`/Engine/EditorBlueprintResources/StandardMacros.IsValid` _left_ptl
    (:`Is Valid`
      (set `/Game/Blueprints/BP_Portal.TargetPortal` _left_ptl (`self.Right_PTL`))
      (set `/Game/Blueprints/BP_Portal.TargetPortal` (`self.Right_PTL`) (`self.Left_PTL`)))
    (:`Is Not Valid`
      _))
  (return _output_get))

(fn `UpdatePortal`
  (params (CurrentPortal :type "/Game/Blueprints/BP_Portal Object Reference"))
  (bind _targetportal (`/Game/Blueprints/BP_Portal.TargetPortal` (`self.CurrentPortal`)))
  (bind _returnvalue (`self.GetActorForwardVector` _targetportal))
  (bind _portalcam (`/Game/Blueprints/BP_Portal.PortalCam` _targetportal))
  (bind _transformcomponent (`PlayerCameraManager.TransformComponent` (`PlayerController.PlayerCameraManager` (`GameplayStatics.GetPlayerController` 0))))
  (bind _output_get (set `self.CurrentPortal` CurrentPortal))
  (bind _targetportal_2 (`/Game/Blueprints/BP_Portal.TargetPortal` _output_get))
  (bind (_returnvalue_roll _returnvalue_pitch _returnvalue_yaw) (`KismetMathLibrary.BreakRotator` (`SceneComponent.K2_GetComponentRotation` (`/Game/Blueprints/BP_Portal.DefaultSceneRoot` _targetportal_2))))
  (bind _returnvalue_2 (`KismetMathLibrary.NormalizedDeltaRotator` (`KismetMathLibrary.MakeRotator` _returnvalue_roll _returnvalue_pitch (- _returnvalue_yaw 180.0)) (`SceneComponent.K2_GetComponentRotation` (`/Game/Blueprints/BP_Portal.DefaultSceneRoot` _output_get))))
  (`SceneComponent.K2_SetWorldLocationAndRotation` (`/Game/Blueprints/BP_Portal.PortalCam` (`/Game/Blueprints/BP_Portal.TargetPortal` (`self.CurrentPortal`))) (+ (`KismetMathLibrary.GreaterGreater_VectorRotator` (`SceneComponent.K2_GetComponentLocation` _transformcomponent) _returnvalue_2) (- (`SceneComponent.K2_GetComponentLocation` (`/Game/Blueprints/BP_Portal.DefaultSceneRoot` _targetportal_2)) (`KismetMathLibrary.GreaterGreater_VectorRotator` (`SceneComponent.K2_GetComponentLocation` (`/Game/Blueprints/BP_Portal.DefaultSceneRoot` _output_get)) _returnvalue_2))) (`KismetMathLibrary.ComposeRotators` (`SceneComponent.K2_GetComponentRotation` _transformcomponent) _returnvalue_2) false false)
  ;[1 1 1] update clipping plane
  (set `SceneCaptureComponent2D.ClipPlaneBase` (+ (`self.K2_GetActorLocation` _targetportal) (* _returnvalue 1.0)) _portalcam)
  (set `SceneCaptureComponent2D.ClipPlaneNormal` _returnvalue _portalcam))

(fn `UserConstructionScript`)