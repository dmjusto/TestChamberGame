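; Procedural room builder actor that tiles a grid mesh into ground, optional ceiling and walls, and box platforms using instanced static mesh components.
; CreateRoom runs from the construction script and BeginPlay, applying mesh, materials and collision before rebuilding, optionally hiding the ceiling in editor.
; AddInstance skips tiles inside EmptyLocations boxes to carve openings, with optional debug boxes.
; An optional text label shows room dimensions in meters.
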(event `self.ReceiveBeginPlay`
  ;[1 1 1] Begin Play
  (`self.CreateRoom` false))

(event `CreateRoom`
  (params (InEditor :type Boolean))
  ;[1 1 1] Create Room: Main function to create room.
  (`TextRenderComponent.SetTextRenderColor` (`self.RoomInfo`) (`self.TextRenderColor`)) ; Update Room Color
  (`self.SetStaticMeshes`) ; Update static meshes.
  (`self.SetMaterials`) ; Update materials
  (`self.SetCollisions`) ; Update Collisions
  (`self.BuildRoomUsingInstancedMeshes` InEditor) ; Build room
  (`self.CreateRoomInfoText`) ; Update room info text
)

(fn `AddInstance`
  (params (InTarget :type "InstancedStaticMeshComponent Object Reference") (InTransform :type "Transform Structure (by ref)"))
  (if (not (`self.IsLocationAtEmptySpace` (.location InTransform)))
    (`InstancedStaticMeshComponent.AddInstance` InTarget InTransform)))

(fn `BuildCeiling`
  (params (Condition :type Boolean))
  (bind _gridsize (`self.GetGridSize`))
  (bind (_roomsize_x _roomsize_y) (break `IntVector` (`self.RoomSize`)))
  (bind (_roomsize_x_2 _roomsize_y_2 _roomsize_z) (break `IntVector` (`self.RoomSize`)))
  (bind _roomsize_x_3 (break `IntVector` (`self.RoomSize`)))
  (`InstancedStaticMeshComponent.ClearInstances` (`self.InstancedStaticMesh_Ceiling`))
  (if (`self.CreateCeiling`)
    (if (not Condition)
      (for _index (range _roomsize_x_3)
        (for _index_2 (range _roomsize_y)
          (`self.AddInstance` (`self.InstancedStaticMesh_Ceiling`) (`KismetMathLibrary.MakeTransform` (`KismetMathLibrary.MakeVector` (`KismetMathLibrary.Conv_IntToDouble` (* _gridsize _index)) (`KismetMathLibrary.Conv_IntToDouble` (* _gridsize _index_2)) (* _roomsize_z (`KismetMathLibrary.Conv_IntToDouble` (`self.GetGridSize`)))))))))))

(fn `BuildGround`
  (bind _gridsize (`self.GetGridSize`))
  (bind _roomsize_x (break `IntVector` (`self.RoomSize`)))
  (bind (_roomsize_x_2 _roomsize_y) (break `IntVector` (`self.RoomSize`)))
  (`InstancedStaticMeshComponent.ClearInstances` (`self.InstancedStaticMesh_Ground`))
  (for _index (range _roomsize_x)
    (for _index_2 (range _roomsize_y)
      (`self.AddInstance` (`self.InstancedStaticMesh_Ground`) (`KismetMathLibrary.MakeTransform` (`KismetMathLibrary.MakeVector` (`KismetMathLibrary.Conv_IntToDouble` (* _index _gridsize)) (`KismetMathLibrary.Conv_IntToDouble` (* _index_2 _gridsize))))))))

(fn `BuildPlatforms`
  (bind (_gridsize _gridsizefloat) (`self.GetGridSize`))
  (if (!= (`KismetArrayLibrary.Array_Length` (`self.Platforms`)) 0)
    (`InstancedStaticMeshComponent.ClearInstances` (`self.InstancedStaticMesh_Platforms`))
    (for _index (range (+ (`KismetArrayLibrary.Array_LastIndex` (`self.Platforms`)) 1))
      (bind (_output_location _output_numberoftiles) (break `/Game/RoomBuilder/Blueprints/RoomBuilderPlatformInfo` (`|GetArrayItem` (`self.Platforms`) _index)))
      (bind (_x _y _z) (break `IntVector` _output_numberoftiles))
      (for _index_2 (range _x)
        (for _index_3 (range _y)
          (for _index_4 (range _z)
            (`self.AddInstance` (`self.InstancedStaticMesh_Platforms`) (`KismetMathLibrary.MakeTransform` (+ _output_location (`KismetMathLibrary.MakeVector` (* _index_2 _gridsizefloat) (* _index_3 _gridsizefloat) (* _index_4 _gridsizefloat)))))))))))

(fn `BuildRoomUsingInstancedMeshes`
  (params (HideCeilingInEditor :type Boolean))
  (`|ExecutionSequence`
    (:`then_0`
      (`self.BuildGround`))
    (:`then_1`
      (`self.BuildCeiling` HideCeilingInEditor))
    (:`then_2`
      (`self.BuildWallsX`))
    (:`then_3`
      (`self.BuildWallsY`))
    (:`then_4`
      (`self.BuildPlatforms`))))

(fn `BuildWallsX`
  (bind (_gridsize _gridsizefloat) (`self.GetGridSize`))
  (bind _roomsize_x (break `IntVector` (`self.RoomSize`)))
  (bind (_roomsize_x_2 _roomsize_y _roomsize_z) (break `IntVector` (`self.RoomSize`)))
  (bind (_roomsize_x_3 _roomsize_y_2) (break `IntVector` (`self.RoomSize`)))
  (`InstancedStaticMeshComponent.ClearInstances` (`self.InstancedStaticMesh_Walls`))
  (if (`self.CreateWalls`)
    (for _index (range _roomsize_x)
      (for _index_2 (range _roomsize_z)
        (bind _returnvalue (`KismetMathLibrary.Conv_IntToDouble` (* _index (`self.GetGridSize`))))
        (bind _returnvalue_2 (`KismetMathLibrary.Conv_IntToDouble` (* _index_2 (`self.GetGridSize`))))
        (`self.AddInstance` (`self.InstancedStaticMesh_Walls`) (`KismetMathLibrary.MakeTransform` (`KismetMathLibrary.MakeVector` _returnvalue 0.0 _returnvalue_2) (struct) (`KismetMathLibrary.MakeVector` 1.0 (`self.XWallScale`) 1.0)))
        (`self.AddInstance` (`self.InstancedStaticMesh_Walls`) (`KismetMathLibrary.MakeTransform` (`KismetMathLibrary.MakeVector` _returnvalue (+ (`KismetMathLibrary.Conv_IntToDouble` (- (* _roomsize_y_2 _gridsize) _gridsize)) _gridsizefloat) _returnvalue_2) (struct :`Pitch` 90.0 :`Yaw` 180.0) (`KismetMathLibrary.MakeVector` 1.0 (`self.XWallScale`) 1.0)))))))

(fn `BuildWallsY`
  (bind (_gridsize _gridsizefloat) (`self.GetGridSize`))
  (bind (_gridsize_2 _gridsizefloat_2) (`self.GetGridSize`))
  (bind (_roomsize_x _roomsize_y) (break `IntVector` (`self.RoomSize`)))
  (bind (_roomsize_x_2 _roomsize_y_2 _roomsize_z) (break `IntVector` (`self.RoomSize`)))
  (bind _roomsize_x_3 (break `IntVector` (`self.RoomSize`)))
  (if (`self.CreateWalls`)
    (for _index (range _roomsize_y)
      (for _index_2 (range _roomsize_z)
        (bind _returnvalue (`KismetMathLibrary.Conv_IntToDouble` (* _index _gridsize_2)))
        (bind _returnvalue_2 (`KismetMathLibrary.Conv_IntToDouble` (* _index_2 (`self.GetGridSize`))))
        (`self.AddInstance` (`self.InstancedStaticMesh_Walls`) (`KismetMathLibrary.MakeTransform` (`KismetMathLibrary.MakeVector` 0.0 _returnvalue _returnvalue_2) (struct) (`KismetMathLibrary.MakeVector` (`self.YWallScale`) 1.0 1.0)))
        (`self.AddInstance` (`self.InstancedStaticMesh_Walls`) (`KismetMathLibrary.MakeTransform` (`KismetMathLibrary.MakeVector` (+ (`KismetMathLibrary.Conv_IntToDouble` (- (* _roomsize_x_3 _gridsize) _gridsize)) _gridsizefloat) (+ _returnvalue _gridsizefloat_2) _returnvalue_2) (struct :`Yaw` 180.0) (`KismetMathLibrary.MakeVector` (`self.YWallScale`) 1.0 1.0)))))))

(fn `CreateRoomInfoText`
  (bind _gridsize (`self.GetGridSize`))
  (bind (_roomsize_x _roomsize_y _roomsize_z) (break `IntVector` (`self.RoomSize`)))
  (bind (_roomsize_x_2 _roomsize_y_2) (break `IntVector` (`self.RoomSize`)))
  (bind (_roomsize_x_3 _roomsize_y_3) (break `IntVector` (`self.RoomSize`)))
  (if (`self.AutomaticTextUpdate`)
    (`TextRenderComponent.K2_SetText` (`self.RoomInfo`) (`|FormatText` "x:{xg}m \ny:{yg}m \nz:{zg}m" (`KismetMathLibrary.SelectFloat` (/ (`KismetMathLibrary.Conv_IntToDouble` (- (* (`self.GetGridSize`) _roomsize_x) (* (`self.GetGridSize`) 2))) 100.0) (/ (`KismetMathLibrary.Conv_IntToDouble` (* (`self.GetGridSize`) _roomsize_x_3)) 100.0) (`self.CreateWalls`)) (`KismetMathLibrary.SelectFloat` (/ (`KismetMathLibrary.Conv_IntToDouble` (- (* (`self.GetGridSize`) _roomsize_y) (* (`self.GetGridSize`) 2))) 100.0) (/ (`KismetMathLibrary.Conv_IntToDouble` (* (`self.GetGridSize`) _roomsize_y_3)) 100.0) (`self.CreateWalls`)) (/ (`KismetMathLibrary.Conv_IntToDouble` (- (* (`self.GetGridSize`) _roomsize_z) (`self.GetGridSize`))) 100.0)))
    (`SceneComponent.K2_SetRelativeLocation` (`self.RoomInfo`) (`KismetMathLibrary.MakeVector` (+ (`KismetMathLibrary.Conv_IntToDouble` (* _gridsize (/ _roomsize_x_2 2))) (`KismetMathLibrary.Conv_IntToDouble` (/ (`self.GetGridSize`) 2))) (+ (`KismetMathLibrary.Conv_IntToDouble` (* _gridsize (/ _roomsize_y_2 2))) (`KismetMathLibrary.Conv_IntToDouble` (/ (`self.GetGridSize`) 2))) (`KismetMathLibrary.Conv_IntToDouble` (+ (`self.GetGridSize`) 5))) false false)))

(fn `GetGridSize`
  (returns (GridSize :type Integer) (GridSizeFloat :type "Float (double-precision)"))
  (bind _gridsize (`self.GridSize`))
  (return _gridsize (`KismetMathLibrary.Conv_IntToDouble` _gridsize)))

(fn `IsLocationAtEmptySpace`
  (params (InLocation :type "Vector Structure (by ref)"))
  (returns (IsInEmpty :type Boolean))
  (locals (Loc_IsInEmptySpace :type Boolean) (PointWorldLocation :type "Vector Structure" :default (0.0 0.0 0.0)))
  (set `local.PointWorldLocation` (+ (`self.K2_GetActorLocation`) InLocation))
  (for _array_element (`self.EmptyLocations`)
    (`|ExecutionSequence`
      (:`then_0`
        (if (`self.DrawEmptyLocationsDebug`)
          (bind (_location _numberoftiles) (break `/Game/RoomBuilder/Blueprints/RoomBuilderEmptyInfo` _array_element))
          (bind (_x _y _z) (break `IntVector` _numberoftiles))
          (bind _returnvalue (* (* (`KismetMathLibrary.MakeVector` (`KismetMathLibrary.Conv_IntToDouble` _x) (`KismetMathLibrary.Conv_IntToDouble` _y) (`KismetMathLibrary.Conv_IntToDouble` _z)) (`KismetMathLibrary.Conv_IntToDouble` (`self.GetGridSize`))) 0.5))
          (bind _returnvalue_2 (+ (`self.K2_GetActorLocation`) _location _returnvalue (-5.0 -5.0 -1.0)))
          (`KismetSystemLibrary.DrawDebugBox` _returnvalue_2 _returnvalue (struct) (struct) 0.1 5.0)))
      (:`then_1`
        (if (`KismetMathLibrary.IsPointInBox` (`local.PointWorldLocation`) _returnvalue_2 _returnvalue)
          (set `local.Loc_IsInEmptySpace` true)))))
  (return (`local.Loc_IsInEmptySpace`)))

(fn `SetCollisions`
  (`PrimitiveComponent.SetCollisionEnabled` (`self.InstancedStaticMesh_Ceiling`) (`self.CollisionType`))
  (`PrimitiveComponent.SetCollisionEnabled` (`self.InstancedStaticMesh_Walls`) (`self.CollisionType`))
  (`PrimitiveComponent.SetCollisionEnabled` (`self.InstancedStaticMesh_Platforms`) (`self.CollisionType`))
  (`PrimitiveComponent.SetCollisionEnabled` (`self.InstancedStaticMesh_Ground`) (`self.CollisionType`)))

(fn `SetMaterials`
  (if (`self.UseSeparateMaterials`)
    (`PrimitiveComponent.SetMaterial` (`self.InstancedStaticMesh_Ceiling`) 0 (`self.CeilingMaterial`))
    (`PrimitiveComponent.SetMaterial` (`self.InstancedStaticMesh_Walls`) 0 (`self.WallsMaterial`))
    (`PrimitiveComponent.SetMaterial` (`self.InstancedStaticMesh_Ground`) 0 (`self.GroundMaterial`))
    (`PrimitiveComponent.SetMaterial` (`self.InstancedStaticMesh_Platforms`) 0 (`self.PlatformsMaterial`))
    (else
      (`PrimitiveComponent.SetMaterial` (`self.InstancedStaticMesh_Ceiling`) 0 (`self.RoomMaterial`))
      (`PrimitiveComponent.SetMaterial` (`self.InstancedStaticMesh_Walls`) 0 (`self.RoomMaterial`))
      (`PrimitiveComponent.SetMaterial` (`self.InstancedStaticMesh_Ground`) 0 (`self.RoomMaterial`))
      (`PrimitiveComponent.SetMaterial` (`self.InstancedStaticMesh_Platforms`) 0 (`self.RoomMaterial`)))))

(fn `SetStaticMeshes`
  (`StaticMeshComponent.SetStaticMesh` (`self.InstancedStaticMesh_Ground`) (`self.GridMesh`))
  (`StaticMeshComponent.SetStaticMesh` (`self.InstancedStaticMesh_Ceiling`) (`self.GridMesh`))
  (`StaticMeshComponent.SetStaticMesh` (`self.InstancedStaticMesh_Walls`) (`self.GridMesh`))
  (`StaticMeshComponent.SetStaticMesh` (`self.InstancedStaticMesh_Platforms`) (`self.GridMesh`)))

(fn `UserConstructionScript`
  (`self.CreateRoom` (`self.HideCeilingInEditor`)))