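; Trigger actor that rumbles the player's gamepad while the player character overlaps it.
; Begin overlap enables force feedback on the first player controller and starts a dynamic force feedback action at full intensity; end overlap stops that same action.
; Both events print debug messages, and a leftover call to stop the FF_PortalFire effect is never executed.
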(event `self.ReceiveActorBeginOverlap`
  (params (OtherActor :type "Actor Object Reference"))
  (bind _returnvalue (`GameplayStatics.GetPlayerController` 0))
  (if (== OtherActor (`GameplayStatics.GetPlayerCharacter` 0))
    (`KismetSystemLibrary.PrintString` "Rumble")
    (set `PlayerController.bForceFeedbackEnabled` true _returnvalue)
    (`PlayerController.PlayDynamicForceFeedback` _returnvalue 1.0 -1.0 true true true true :!label _label)))

(event `self.ReceiveActorEndOverlap`
  (params (OtherActor :type "Actor Object Reference"))
  (if (== OtherActor (`GameplayStatics.GetPlayerCharacter` 0))
    (`KismetSystemLibrary.PrintString` "stop rumble" true true (struct :`R` 1.0 :`G` 0.003465 :`A` 1.0))
    (goto _label :!via `Stop`)))

(fn `UserConstructionScript`)