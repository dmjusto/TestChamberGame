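; Portal manager that places a linked pair of portals where the player aims, driven by left and right events bound on FirstPersonCharacter.
; SpawnPortal line-traces from the camera, replaces that side's portal and orients it to the surface, yawing to the player on floors and ceilings.
; SetTarget links the pair or self-targets a lone portal, while timelines scale it open.
; Uncalled helpers here handle render-target setup and player-relative capture cameras with clip planes.
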(event `self.ReceiveTick`
  (params (DeltaSeconds :type "Float (single-precision)"))
  ;[1 1 1] Tick Event
)

(event `LeftPortalCustomEvent`
  (bind _left_ptl (`self.Left_PTL`))
  (bind _returnvalue_x (`KismetMathLibrary.BreakVector` (`self.GetActorScale3D` _left_ptl)))
  ;[1 0.8691 0.2429] Make Left Portal
  (bind _spawnedportal (`self.SpawnPortal` (`self.Left_PTL`) (`self.Right_PTL`)))
  (`PrimitiveComponent.SetMaterial` (`/Game/MyBlueprints/BP_Portal.RingMesh` _spawnedportal) 0 "/Game/MyMaterials/PortalRingRedMat.PortalRingRedMat")
  (bind _output_get (set `self.Left_PTL` _spawnedportal))
  (bind _output_get_2 (set `self.Portal_1` _output_get))
  (`self.SetTarget` _output_get_2 (`self.Portal_2`))
  (bind (_direction _portal_opening) (`Timeline|OpenPortal 1` :!via `PlayFromStart`)
    (:`Update`
      (`self.SetActorScale3D` _left_ptl (`KismetMathLibrary.MakeVector` _returnvalue_x _portal_opening _portal_opening)))))

(event `self.ReceiveBeginPlay`
  (bind _asfirst_person_character (cast `/Game/FirstPersonBP/Blueprints/FirstPersonCharacter` (`GameplayStatics.GetPlayerCharacter` 0) :!pure true))
  (`|ExecutionSequence`
    (:`then_0`
      (add `/Game/FirstPersonBP/Blueprints/FirstPersonCharacter.CreateLeftPortal` _asfirst_person_character (delegate `LeftPortalCustomEvent`)))
    (:`then_1`
      (add `/Game/FirstPersonBP/Blueprints/FirstPersonCharacter.CreateRightPortal` _asfirst_person_character (delegate `RightPortalCustomEvent`)))))

(event `RightPortalCustomEvent`
  (bind _returnvalue_x (`KismetMathLibrary.BreakVector` (`self.GetActorScale3D` (`self.Right_PTL`))))
  ;[0.1576 0.1835 1] Make Right Portal
  (bind _spawnedportal (`self.SpawnPortal` (`self.Right_PTL`) (`self.Left_PTL`)))
  (bind _output_get (set `self.Right_PTL` _spawnedportal))
  (bind _output_get_2 (set `self.Portal_2` _output_get))
  (`self.SetTarget` _output_get_2 (`self.Portal_1`))
  (bind (_direction _portal_opening) (`Timeline|OpenPortal` :!via `PlayFromStart`)
    (:`Update`
      (`self.SetActorScale3D` (`self.Right_PTL`) (`KismetMathLibrary.MakeVector` _returnvalue_x _portal_opening _portal_opening)))))

(fn `InitializeSceneCapture`
  (params (ThisPortal :type "/Game/MyBlueprints/BP_Portal Object Reference") (OtherPortal :type "/Game/MyBlueprints/BP_Portal Object Reference"))
  (locals (Current :type "/Game/MyBlueprints/BP_Portal Object Reference") (Other :type "/Game/MyBlueprints/BP_Portal Object Reference"))
  (set `local.Other` OtherPortal)
  (set `local.Current` ThisPortal)
  (set `self.RenderTarget` (`|GetArrayItem` (`/Game/MyBlueprints/BP_Portal.RenderTargets` (`local.Current`))))
  (`/Engine/EditorBlueprintResources/StandardMacros.IsValid` (`local.Other`)
    (:`Is Valid`
      (set `SceneCaptureComponent2D.TextureTarget` (`self.RenderTarget`) (`/Game/MyBlueprints/BP_Portal.PortalCam` (`local.Other`))))
    (:`Is Not Valid`
      (set `SceneCaptureComponent2D.TextureTarget` (`self.RenderTarget`) (`/Game/MyBlueprints/BP_Portal.PortalCam` (`local.Current`)))))
  (bind _returnvalue (`PrimitiveComponent.CreateDynamicMaterialInstance` (`/Game/MyBlueprints/BP_Portal.MeshP` (`local.Current`)) 0 null "None"))
  (`MaterialInstanceDynamic.SetTextureParameterValue` _returnvalue "TextureRT" (`self.RenderTarget`)))

(fn `SetTarget`
  (params (thisPortal :type "/Game/MyBlueprints/BP_Portal Object Reference") (target :type "/Game/MyBlueprints/BP_Portal Object Reference"))
  (bind _mesh (`Character.Mesh` (`GameplayStatics.GetPlayerCharacter` 0)))
  (`/Engine/EditorBlueprintResources/StandardMacros.IsValid` target
    (:`Is Valid`
      ;[0.2991 0.4184 1] Set the other portal as this portal's target
      (bind _output_get (set `/Game/MyBlueprints/BP_Portal.TargetPortal` target thisPortal))
      (set `/Game/MyBlueprints/BP_Portal.TargetPortal` thisPortal _output_get)
      (`SceneComponent.SetVisibility` _mesh true false))
    (:`Is Not Valid`
      ;[0.3219 1 0.6725] set itself as its target if the other portal does not exist yet
      (set `/Game/MyBlueprints/BP_Portal.TargetPortal` thisPortal thisPortal)
      (`SceneComponent.SetVisibility` _mesh false false))))

(fn `SpawnPortal`
  (params (TypeToSpawn :type "/Game/MyBlueprints/BP_Portal Object Reference") (TargetType :type "/Game/MyBlueprints/BP_Portal Object Reference"))
  (returns (SpawnedPortal :type "/Game/MyBlueprints/BP_Portal Object Reference"))
  (locals (PortalType :type "/Game/MyBlueprints/BP_Portal Object Reference") (HitSurface :type "Actor Object Reference") (Target :type "/Game/MyBlueprints/BP_Portal Object Reference") (Spawn :type "/Game/MyBlueprints/BP_Portal Object Reference"))
  (bind _playercameramanager (`PlayerController.PlayerCameraManager` (`GameplayStatics.GetPlayerController` 0)))
  (bind _returnvalue (`PlayerCameraManager.GetCameraLocation` _playercameramanager))
  (bind (_returnvalue_roll _returnvalue_pitch _returnvalue_yaw) (`KismetMathLibrary.BreakRotator` (`SceneComponent.K2_GetComponentRotation` (`PlayerCameraManager.TransformComponent` (`PlayerController.PlayerCameraManager` (`GameplayStatics.GetPlayerController` 0))))))
  ;[1 0.2212 0.9138] fire line trace
  (set `local.PortalType` TypeToSpawn)
  (set `local.Target` TargetType)
  (bind _outhit (`KismetSystemLibrary.LineTraceSingle` _returnvalue (+ (* (`KismetMathLibrary.GetForwardVector` (`PlayerCameraManager.GetCameraRotation` _playercameramanager)) 10000.0) _returnvalue) "TraceTypeQuery1"))
  (set `local.HitSurface` (`.HitActor` (`GameplayStatics.BreakHitResult` _outhit)))
  (`/Engine/EditorBlueprintResources/StandardMacros.IsValid` (`local.PortalType`)
    (:`Is Valid`
      (`self.K2_DestroyActor` (`local.PortalType`)))
    (:`Is Not Valid`
      _))
  (bind _returnvalue_2 (`KismetMathLibrary.Conv_VectorToRotator` (`.ImpactNormal` (`GameplayStatics.BreakHitResult` _outhit))))
  (bind _returnvalue_3 (`|SpawnActorFromClass` "/Game/MyBlueprints/BP_Portal.BP_Portal_C" (`KismetMathLibrary.MakeTransform` (+ (`.ImpactPoint` (`GameplayStatics.BreakHitResult` _outhit)) (* (`.ImpactNormal` (`GameplayStatics.BreakHitResult` _outhit)) 0.02)) _returnvalue_2 (1.0 0.2 0.2)) "Undefined" "OverrideRootScale" null null null))
  (bind _output_get (set `local.Spawn` _returnvalue_3))
  (bind _z (.z (`.ImpactNormal` (`GameplayStatics.BreakHitResult` _outhit))))
  ;[0.4306 1 0.09746] Orient the portal to the player if it is spawned on the ground or ceiling
  (if (== (`KismetMathLibrary.Abs` _z) 1.0)
    (`SceneComponent.K2_SetWorldRotation` (`Actor.RootComponent` (`local.Spawn`)) (`KismetMathLibrary.MakeRotator` (.roll _returnvalue_2) (.pitch _returnvalue_2) (+ _returnvalue_yaw (* (`KismetMathLibrary.FClamp` _z) 180.0))) false false))
  (set `/Game/MyBlueprints/BP_Portal.PortalSurface` (`local.HitSurface`) _output_get)
  (`/Engine/EditorBlueprintResources/StandardMacros.IsValid` (`local.Target`)
    (:`Is Valid`
      (set `/Game/MyBlueprints/BP_Portal.TargetPortal` (`local.Target`) (`local.Spawn`))
      (set `/Game/MyBlueprints/BP_Portal.TargetPortal` (`local.Spawn`) (`local.Target`)))
    (:`Is Not Valid`
      _))
  (return (`local.Spawn`)))

(fn `UpdatePortal`
  (params (CurrentPortal :type "/Game/MyBlueprints/BP_Portal Object Reference"))
  (bind _targetportal (`/Game/MyBlueprints/BP_Portal.TargetPortal` (`self.CurrentPortal`)))
  (bind _returnvalue (`self.GetActorForwardVector` _targetportal))
  (bind _transformcomponent (`PlayerCameraManager.TransformComponent` (`PlayerController.PlayerCameraManager` (`GameplayStatics.GetPlayerController` 0))))
  (bind _portalcam (`/Game/MyBlueprints/BP_Portal.PortalCam` _targetportal))
  (bind _output_get (set `self.CurrentPortal` CurrentPortal))
  (bind _defaultsceneroot (`/Game/MyBlueprints/BP_Portal.DefaultSceneRoot` (`/Game/MyBlueprints/BP_Portal.TargetPortal` _output_get)))
  (bind (_returnvalue_roll _returnvalue_pitch _returnvalue_yaw) (`KismetMathLibrary.BreakRotator` (`SceneComponent.K2_GetComponentRotation` _defaultsceneroot)))
  (bind _returnvalue_2 (`KismetMathLibrary.NormalizedDeltaRotator` (`KismetMathLibrary.MakeRotator` _returnvalue_roll _returnvalue_pitch (- _returnvalue_yaw 180.0)) (`SceneComponent.K2_GetComponentRotation` (`/Game/MyBlueprints/BP_Portal.DefaultSceneRoot` _output_get))))
  (`SceneComponent.K2_SetWorldLocationAndRotation` (`/Game/MyBlueprints/BP_Portal.PortalCam` (`/Game/MyBlueprints/BP_Portal.TargetPortal` (`self.CurrentPortal`))) (+ (`KismetMathLibrary.GreaterGreater_VectorRotator` (`SceneComponent.K2_GetComponentLocation` _transformcomponent) _returnvalue_2) (- (`SceneComponent.K2_GetComponentLocation` _defaultsceneroot) (`KismetMathLibrary.GreaterGreater_VectorRotator` (`SceneComponent.K2_GetComponentLocation` (`/Game/MyBlueprints/BP_Portal.DefaultSceneRoot` _output_get)) _returnvalue_2))) (`KismetMathLibrary.ComposeRotators` (`SceneComponent.K2_GetComponentRotation` _transformcomponent) _returnvalue_2) false false)
  ;[1 1 1] update clipping plane
  (set `SceneCaptureComponent2D.ClipPlaneBase` (+ (`self.K2_GetActorLocation` _targetportal) (* _returnvalue 1.0)) _portalcam)
  (set `SceneCaptureComponent2D.ClipPlaneNormal` _returnvalue _portalcam))

(fn `UserConstructionScript`)