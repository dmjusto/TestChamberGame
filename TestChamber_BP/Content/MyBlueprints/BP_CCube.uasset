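; BP_CCube is a cube the first-person player can pick up while overlapping it and throw.
; On BeginPlay it binds to the character's pickup and drop events and creates normal and transparent dynamic materials.
; Pickup disables physics, attaches to the character's CubeLocator and turns the cube transparent.
; Release re-enables physics, detaches, moves it to the character's Sphere, launches it forward and restores the normal material.
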(event `ReleaseCube`
  (bind _cubemesh (`self.CubeMesh`))
  ;[1 1 1] Cube Relesea
  (if (`self.IsHeld`)
    (`KismetSystemLibrary.PrintString` "Dropped the cube!" true true (struct :`R` 1.0 :`B` 0.022459 :`A` 1.0))
    (`PrimitiveComponent.SetSimulatePhysics` (`self.CubeMesh`) true)
    (`self.K2_DetachFromActor` "KeepWorld" "KeepWorld" "KeepWorld")
    (bind _asfirst_person_character (cast `/Game/FirstPersonBP/Blueprints/FirstPersonCharacter` (`GameplayStatics.GetPlayerCharacter` 0)))
    (bind (_returnvalue_location _returnvalue_rotation) (`KismetMathLibrary.BreakTransform` (`SceneComponent.K2_GetComponentToWorld` (`/Game/FirstPersonBP/Blueprints/FirstPersonCharacter.Sphere` _asfirst_person_character))))
    (`SceneComponent.K2_SetWorldLocationAndRotation` (`self.CubeMesh`) _returnvalue_location _returnvalue_rotation false false)
    (`PrimitiveComponent.AddImpulse` _cubemesh (* (`SceneComponent.GetForwardVector` _cubemesh) (`self.ReleaseForce`)) "None" true)
    (`PrimitiveComponent.SetMaterial` (`self.CubeMesh`) 0 (`self.NormalMat`))
    (set `self.IsHeld` false)))

(event `PickUpCube`
  ;[1 1 1] Cube Pickup
  (if (`self.IsGrabable`)
    (`PrimitiveComponent.SetSimulatePhysics` (`self.CubeMesh`) false)
    (bind _asfirst_person_character (cast `/Game/FirstPersonBP/Blueprints/FirstPersonCharacter` (`GameplayStatics.GetPlayerCharacter` 0)))
    (`self.K2_AttachToComponent` (`/Game/FirstPersonBP/Blueprints/FirstPersonCharacter.CubeLocator` _asfirst_person_character) "None" "SnapToTarget" "SnapToTarget" "KeepRelative")
    (`PrimitiveComponent.SetMaterial` (`self.CubeMesh`) 0 (`self.TransparentMat`))
    (set `self.IsHeld` true)))

(event `self.ReceiveBeginPlay`
  (bind _asfirst_person_character (cast `/Game/FirstPersonBP/Blueprints/FirstPersonCharacter` (`GameplayStatics.GetPlayerCharacter` 0) :!pure true))
  (add `/Game/FirstPersonBP/Blueprints/FirstPersonCharacter.PickupCubeEvent` _asfirst_person_character (delegate `PickUpCube`))
  (add `/Game/FirstPersonBP/Blueprints/FirstPersonCharacter.DropCubeEvent` _asfirst_person_character (delegate `ReleaseCube`))
  (bind _returnvalue (`PrimitiveComponent.CreateDynamicMaterialInstance` (`self.CubeMesh`) 0 "/Game/MyMaterials/yellowMat.yellowMat" "None"))
  (set `self.NormalMat` _returnvalue)
  (bind _returnvalue_2 (`PrimitiveComponent.CreateDynamicMaterialInstance` (`self.CubeMesh`) 0 "/Game/MyMaterials/yellowMat1.yellowMat1" "None"))
  (set `self.TransparentMat` _returnvalue_2)
  (`PrimitiveComponent.SetMaterial` (`self.CubeMesh`) 0 (`self.NormalMat`)))

(event `self.ReceiveActorBeginOverlap`
  (params (OtherActor :type "Actor Object Reference"))
  (cast `/Game/FirstPersonBP/Blueprints/FirstPersonCharacter` OtherActor)
  (set `self.IsGrabable` true))

(event `self.ReceiveActorEndOverlap`
  (params (OtherActor :type "Actor Object Reference"))
  (set `self.IsGrabable` false))

(fn `UserConstructionScript`)